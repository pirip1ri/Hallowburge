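; Shooting enemy astronaut character that supplies movement speeds, combat ranges and a patrol route, and reports state changes to its AI controller.
; Attacks play a montage whose notify line-traces toward the controller's target before shooting.
; Damage first checks for possession, otherwise reducing health and playing a hit montage before returning to attacking.
; Death ragdolls the mesh and stops AI logic; unpossessing stuns the released character.
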(event EventBeginPlay
  (bind _health (Variables|Default|GetHealth))
  (Variables|/Script/Hallowburge.HealthComponent|SetMaxHealth _health 2.0)
  (Development|PrintString (Utilities|String|ToString(Float) (Variables|/Script/Hallowburge.HealthComponent|GetCurrentHealth _health)))
  (bind _asaic_enemy_test_controller_base (Utilities|Casting|CastToAIC_EnemyTestControllerBase (AI|GetAIController self)))
  (Variables|Default|SetAICEnemyBase _asaic_enemy_test_controller_base))

(event EventOnUnpossessCharacterinScene
  (params (PossessedCharacter :type Possessable%20Character%20Object%20Reference))
  (bind _asaic_enemy_test_controller_base (Utilities|Casting|CastToAIC_EnemyTestControllerBase (AI|GetAIController PossessedCharacter)))
  (Utilities|IsValid _asaic_enemy_test_controller_base
    (:Is%20Valid
      (Default|SetStateasStunned _asaic_enemy_test_controller_base))))

(event EventTick
  (params (DeltaSeconds :type Float%20%28single-precision%29))
  (Variables|Default|SetDestinationDistanceFromSelf (Math|Vector|Distance(Vector) (Variables|Default|GetDestination) (Transformation|GetActorLocation))))

(event EventDefaultAttack
  (|AttackFunctionality))

(event EventJumptoDestination
  (params (Destination :type Vector :default "0, 0, 0"))
  (|JumpFunctionality Destination))

(event EventOnDeath
  (|DeathFunctionality))

(event Game|Damage|EventAnyDamage
  (params (Damage :type Float%20%28single-precision%29) (DamageType :type Damage%20Type%20Object%20Reference) (InstigatedBy :type Controller%20Object%20Reference) (DamageCauser :type Actor%20Object%20Reference))
  (|CheckToSeeIfTheCharacterIsPossessed
    (:then
      ;[1 1 1] Leave Possessed Enemy
      (Class|PossessableCharacter|PossessionAbilityCheck))
    (:else
      (|NormalDamageFunctionality Damage))))

(fn ConstructionScript
  (|CallParentFunction))

(fn SetMovementSpeed
  (params (Speed :type E_MovementSpeed%20Enum :default "NewEnumerator0"))
  (bind _output_get (Variables|/Script/Engine.CharacterMovementComponent|SetMaxWalkSpeed (Variables|Character|GetCharacterMovement) (Utilities|Select :Index Speed :NewEnumerator0 0.0 :NewEnumerator1 3e+02 :NewEnumerator2 6e+02 :NewEnumerator3 8e+02)))
  (return _output_get))

(fn GetIdealRange
  (return 7e+02 6e+02))

(fn GetPatrolRoute
  (return (Variables|Default|GetPatrolRoute)))