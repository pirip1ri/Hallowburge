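; Player controller for the ghost character that handles aim and crouch input.
; Aiming switches the character from movement-oriented to controller-desired rotation while a timeline slides the camera to an over-the-shoulder offset.
; Crouching lowers walk speed and drives the spring arm's height through a second timeline.
; Releasing either input restores movement settings and reverses its timeline for a smooth return.
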(event Input|EnhancedActionEvents|EnhancedInputActionIA_Aim
  (params (ActionValue :type Boolean) (ElapsedSeconds :type Float%20%28double-precision%29) (TriggeredSeconds :type Float%20%28double-precision%29) (InputAction :type Input%20Action%20Object%20Reference :default "/Game/Blueprints/PlayerCharacter/Inputs/IA_Aim.IA_Aim"))
  (:Triggered
    (|AimFunctions :!label _label))
  (:Completed
    (goto _label execute2)))

(event Input|EnhancedActionEvents|EnhancedInputActionIA_CrouchAction
  (params (ActionValue :type Boolean) (ElapsedSeconds :type Float%20%28double-precision%29) (TriggeredSeconds :type Float%20%28double-precision%29) (InputAction :type Input%20Action%20Object%20Reference :default "/Game/Blueprints/PlayerCharacter/Inputs/IA_CrouchAction.IA_CrouchAction"))
  (:Triggered
    (|CrouchFunction :!label _label))
  (:Completed
    (goto _label execute2)))

(event EventBeginPlay
  (bind _asbp_ghost_character (Utilities|Casting|CastToBP_GhostCharacter (Pawn|GetControlledPawn)))
  (Variables|Default|SetCharacter%20Movement (Variables|/Script/Engine.Character|GetCharacterMovement _asbp_ghost_character))
  (Variables|Default|SetIsAiming false))

(event EventTick
  (params (DeltaSeconds :type Float%20%28single-precision%29)))

(fn ConstructionScript)

(fn SetCameraLocation
  (params (Alpha :type Float%20%28single-precision%29))
  (bind _asbp_ghost_character (Utilities|Casting|CastToBP_GhostCharacter (Pawn|GetControlledPawn)))
  (Transformation|SetRelativeLocation (Variables|/Script/Hallowburge.GhostPlayerCharacter|GetCamera _asbp_ghost_character) (Math|Vector|Lerp(Vector) "0, 0, 0" "125.000000,55.000000,50.000000" Alpha) false false))

(fn SetAimTrue
  (params (self2 :type Character%20Movement%20Component%20Object%20Reference) (self3 :type Character%20Movement%20Component%20Object%20Reference))
  (Variables|Default|SetIsAiming true)
  (Variables|/Script/Engine.CharacterMovementComponent|SetbOrientRotationToMovement self3 false)
  (Variables|/Script/Engine.CharacterMovementComponent|SetbUseControllerDesiredRotation self2 true))

(fn SetAimFalse
  (params (self2 :type Character%20Movement%20Component%20Object%20Reference) (self3 :type Character%20Movement%20Component%20Object%20Reference))
  (Variables|Default|SetIsAiming false)
  (Variables|/Script/Engine.CharacterMovementComponent|SetbOrientRotationToMovement self3 true)
  (Variables|/Script/Engine.CharacterMovementComponent|SetbUseControllerDesiredRotation self2 false))